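; BP_DebugText is an actor that configures Wi-Fi auto-connect on a Pico XR headset, despite its debug-text name.
; On BeginPlay it reads SSID and password from config.txt, accepting only four comma-separated fields.
; It clears the auto-connect Wi-Fi, then sets the new one both immediately and again from the clear callback.
; SetWidgetText recolors and updates a WBP_SimpleText widget but is not called here.
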(event Custom|CustomEvent_1
  (params (Result :type Boolean))
  (Class|PicoXRSystemAPI|PXRSetAutoConnectWifi (Variables|Default|GetPicoXRSystemAPI) (Variables|Default|GetSSID) (Variables|Default|GetPassword) 0 (delegate Custom|CustomEvent_0)))

(event Custom|CustomEvent_0
  (params (Result :type Boolean)))

(event EventBeginPlay
  (Utilities|FlowControl|Sequence
    (:then_0
      (CallFunction|LoadConfiguration))
    (:then_1
      (Class|PicoXRSystemAPI|PXRClearAutoConnectWifi (Variables|Default|GetPicoXRSystemAPI) (delegate Custom|CustomEvent_1)))
    (:then_2
      (Class|PicoXRSystemAPI|PXRSetAutoConnectWifi (Variables|Default|GetPicoXRSystemAPI) (Variables|Default|GetSSID) (Variables|Default|GetPassword) 0 (delegate Custom|CustomEvent_0)))))

(event Collision|EventActorBeginOverlap
  (params (OtherActor :type Actor%20Object%20Reference)))

(event EventTick
  (params (DeltaSeconds :type Float%20%28single-precision%29)))

(fn ConstructionScript)

(fn SetWidgetText
  (params (text :type String))
  (bind _aswbp_simple_text (Utilities|Casting|CastToWBP_SimpleText (UserInterface|GetUserWidgetObject (Variables|Default|GetWidget))))
  (Default|ChangeText _aswbp_simple_text text)
  (Appearance|SetColorandOpacity _aswbp_simple_text "(R=0.149424,G=0.113816,B=1.000000,A=1.000000)" :!class /Script/UMG.UserWidget))

(fn LoadConfiguration
  (bind _returnvalue (Class|TMCFIleController|LoadFiletoString "config.txt"))
  (if (== (Utilities|Array|Length (Utilities|String|ParseIntoArray _returnvalue "," false)) 4)
    (Utilities|FlowControl|Sequence
      (:then_0
        (Variables|Default|SetSSID (Utilities|Array|Get(acopy) (Utilities|String|ParseIntoArray _returnvalue "," false))))
      (:then_1
        (Variables|Default|SetPassword (Utilities|Array|Get(acopy) (Utilities|String|ParseIntoArray _returnvalue "," false) 1))))))